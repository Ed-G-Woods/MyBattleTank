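; Player-controllable tank pawn Blueprint that wires up movement, aiming, camera orbit, firing and an HP widget.
; BeginPlay hands barrel and turret to the aiming component and both tracks to the movement component, then gives the HP widget a reference to the tank.
; Input rotates the gimbal and spring arm, throttles each track directly or drives intended move and turn through TankMovement, and triggers Fire.
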(event `self.ReceiveBeginPlay`
  (`TankAimmingComponent.TankAimmingComponentSetup` (`self.TankAimmingComponent`) (`self.TankBarrel`) (`self.TankTurret`))
  (`TankMovementComponent.Initialise` (`self.TankMovement`) (`self.TankTrack_L`) (`self.TankTrack_R`))
  (bind _ashp (cast `/Game/UI/HP` (`WidgetComponent.GetUserWidgetObject` (`self.Widget`))))
  (set `/Game/UI/HP.Tank` self _ashp))

(event `self.ReceiveTick`
  (params (DeltaSeconds :type "Float (single-precision)")))

(event `InputAxis|turn X`
  (params (AxisValue :type "Float (single-precision)"))
  (`SceneComponent.K2_AddLocalRotation` (`self.X Gimbal`) (`KismetMathLibrary.MakeRotator` 0.0 0.0 AxisValue) false false))

(event `InputAxis|turn Y`
  (params (AxisValue :type "Float (single-precision)"))
  (`SceneComponent.K2_AddLocalRotation` (`self.SpringArm`) (`KismetMathLibrary.MakeRotator` 0.0 AxisValue) false false))

(event `InputAxis|Left Track`
  (params (AxisValue :type "Float (single-precision)"))
  (`TankTrack.SetThrottle` (`self.TankTrack_L`) AxisValue))

(event `InputAction|Fire`
  (params (Key :type "Key Structure"))
  (:`Pressed`
    (`self.Fire`)))

(event `InputAxis|Right Track`
  (params (AxisValue :type "Float (single-precision)"))
  (`TankTrack.SetThrottle` (`self.TankTrack_R`) AxisValue))

(event `InputAxis|WS`
  (params (AxisValue :type "Float (single-precision)"))
  (`TankMovementComponent.IntendMoveForward` (`self.TankMovement`) AxisValue))

(event `InputAxis|AD`
  (params (AxisValue :type "Float (single-precision)"))
  (`TankMovementComponent.IntendToTurn` (`self.TankMovement`) AxisValue))

(fn `UserConstructionScript`
  (set `self.TankAimmingComponent` (`self.TankAimming`)))